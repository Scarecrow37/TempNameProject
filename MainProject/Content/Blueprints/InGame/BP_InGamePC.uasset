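; In-game player controller that handles input and HUD updates for chat, sound settings and ink switching.
; Enter focuses the chat box in UI-only mode, while M toggles the in-game widget and sets cursor and input mode from its sound panel visibility.
; Right mouse cycles the PlayerState's brush texture through its material list, then refreshes the widget's ink.
; A user-name update event refreshes the widget after a short delay.
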(event `self.OnUpdateUserName`
  (params (UserName :type String))
  (`KismetSystemLibrary.Delay` 0.1)
  (bind _aswbp_in_game_widget (cast `/Game/Blueprints/InGame/WBP_InGameWidget` (`self.InGameWidget`))
    (:`then`
      (`InGameUserWidget.UpdateInGameUserName` _aswbp_in_game_widget))
    (:`CastFailed`
      (`KismetSystemLibrary.PrintString` "[ LobbyPC ] InGame Widget Cast Failed !!!"))))

(event `Key|Enter`
  (params (Key :type "Key Structure"))
  (bind _returnvalue (`GameplayStatics.GetPlayerController` 0))
  (:`Pressed`
    (`Widget.SetKeyboardFocus` (`ChatWidget.ChatInputTextBox` (`self.ChatWidget`)))
    (set `PlayerController.bShowMouseCursor` true _returnvalue)
    (`WidgetBlueprintLibrary.SetInputMode_UIOnlyEx` _returnvalue null)))

(event `Key|M`
  (params (Key :type "Key Structure"))
  (bind _returnvalue (`GameplayStatics.GetPlayerController` 0))
  (bind _returnvalue_2 (`GameplayStatics.GetPlayerController` 0))
  (bind _ingamewidget (`self.InGameWidget`))
  (:`Pressed`
    (`InGameUserWidget.ToggleVisibleWidget` _ingamewidget)
    (bind _returnvalue_3 (`InGameUserWidget.InGameSoundISVisible` _ingamewidget))
    (if _returnvalue_3
      (set `PlayerController.bShowMouseCursor` true _returnvalue_2)
      (`WidgetBlueprintLibrary.SetInputMode_GameAndUIEx` _returnvalue_2 (`self.InGameWidget`))
      (else
        (set `PlayerController.bShowMouseCursor` false _returnvalue)
        (`WidgetBlueprintLibrary.SetInputMode_GameOnly` _returnvalue)))))

(event `Key|RightMouseButton`
  (params (Key :type "Key Structure"))
  (:`Pressed`
    (`self.UpdateChangeInk`)))

(fn `UpdateChangeInk`
  (bind _asbp_player_state (cast `/CharacterPlugin/Blueprints/Gamemodes/BP_PlayerState` (`GameplayStatics.GetPlayerState` 0)))
  (bind _result (`/Engine/EditorBlueprintResources/StandardMacros.IncrementInt` (`/CharacterPlugin/Blueprints/Gamemodes/BP_PlayerState.CurrentTexture` _asbp_player_state))
    (:`  `
      (if (== _result (`KismetArrayLibrary.Array_Length` (`/CharacterPlugin/Blueprints/Gamemodes/BP_PlayerState.MaterialList` _asbp_player_state)))
        (`/CharacterPlugin/Blueprints/Gamemodes/BP_PlayerState.CallChangeBrushTexture` _asbp_player_state 0)
        (else
          (`/CharacterPlugin/Blueprints/Gamemodes/BP_PlayerState.CallChangeBrushTexture` _asbp_player_state _result)))
      (bind _aswbp_in_game_widget (cast `/Game/Blueprints/InGame/WBP_InGameWidget` (`self.InGameWidget`)))
      (`/Game/Blueprints/InGame/WBP_InGameWidget.ChangeInk` _aswbp_in_game_widget))))

(fn `UserConstructionScript`)